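; Blueprint function library with messaging and tag helpers for the Behavior Toolkit's AI.
; SendAreaMessage broadcasts through AI hearing as a noise event, using the message enum name as tag and the radius as loudness over a unit max range.
; SendDirectMessage passes the message straight to the receiving AI's BP_BehaviorComponent.
; CompareTags returns true when two actors share any actor tag.
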(fn `CompareTags`
  (params (FirstActor :type "Actor Object Reference") (SecondActor :type "Actor Object Reference"))
  (returns (HasSimilar :type Boolean))
  (bind _secondactor (`local.SecondActor`))
  (for _array_element (`Actor.Tags` FirstActor)
    (`/Engine/EditorBlueprintResources/StandardMacros.IsValid` _secondactor
      (:`Is Valid`
        (if (>= (`KismetArrayLibrary.Array_Find` (`Actor.Tags` _secondactor) _array_element) 0)
          (return true)))))
  (return false))

(fn `SendAreaMessage`
  (params (OriginLocation :type "Vector Structure") (Radius :type "Float (double-precision)") (Instigator :type "Actor Object Reference") (MessageToSend :type "/Game/BehaviorToolkit/Blueprints/Enums/Enum_MessageTag Enum" :default "NewEnumerator3"))
  (`AISense_Hearing.ReportNoiseEvent` null OriginLocation Radius Instigator 1.0 (`|GetEnumeratorName` MessageToSend)))

(fn `SendDirectMessage`
  (params (ReceivingAI :type "Actor Object Reference") (MessageToSend :type "/Game/BehaviorToolkit/Blueprints/Enums/Enum_MessageTag Enum" :default "NewEnumerator3"))
  (bind _output (`|GetArrayItem` (`Actor.K2_GetComponentsByClass` ReceivingAI "/Game/BehaviorToolkit/Blueprints/BP_BehaviorComponent.BP_BehaviorComponent_C")))
  (`/Engine/EditorBlueprintResources/StandardMacros.IsValid` _output
    (:`Is Valid`
      (`/Game/BehaviorToolkit/Blueprints/BP_BehaviorComponent.ReceiveMessageTag` _output MessageToSend))))