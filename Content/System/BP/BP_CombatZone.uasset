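; BP_CombatZone is a trigger actor that starts the final combat phase when the player's ThirdPersonCharacter enters it.
; Overlapping Box calls FinalObjective on the character, moves Cube to its relative origin and calls SwitchMode on every BP_MasterAI.
; Overlapping Box1 offsets Cube sideways, apparently as a barrier or door.
; Each trigger has its own DoOnce, and Cube moves instantly without sweep.
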(event `self.Box.OnComponentBeginOverlap`
  (params (OverlappedComponent :type "PrimitiveComponent Object Reference") (OtherActor :type "Actor Object Reference") (OtherComp :type "PrimitiveComponent Object Reference") (OtherBodyIndex :type Integer) (bFromSweep :type Boolean) (SweepResult :type "HitResult Structure (by ref)"))
  (bind _asthird_person_character (cast `/Game/System/BP/ThirdPersonCharacter` OtherActor))
  (`/Engine/EditorBlueprintResources/StandardMacros.DoOnce` false
    (:`Completed`
      (`/Game/System/BP/ThirdPersonCharacter.Final Objective` _asthird_person_character)
      (`SceneComponent.K2_SetRelativeLocation` (`self.Cube`) (0.0 0.0 0.0) false false)
      (bind _outactors (`GameplayStatics.GetAllActorsOfClass` "/Game/System/BP/BP_MasterAI.BP_MasterAI_C"))
      (`/Game/System/BP/BP_MasterAI.Switch Mode` _outactors true))))

(event `self.Box1.OnComponentBeginOverlap`
  (params (OverlappedComponent :type "PrimitiveComponent Object Reference") (OtherActor :type "Actor Object Reference") (OtherComp :type "PrimitiveComponent Object Reference") (OtherBodyIndex :type Integer) (bFromSweep :type Boolean) (SweepResult :type "HitResult Structure (by ref)"))
  (cast `/Game/System/BP/ThirdPersonCharacter` OtherActor)
  (`/Engine/EditorBlueprintResources/StandardMacros.DoOnce` false
    (:`Completed`
      (`SceneComponent.K2_SetRelativeLocation` (`self.Cube`) (0.0 -280.0 0.0) false false))))

(fn `UserConstructionScript`)