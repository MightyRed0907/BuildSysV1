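; Base melee enemy character that wanders randomly until switched into combat, then chases and attacks the player.
; A timer and AIMoveTo loop drives movement, while SwitchMode sets walk or sprint speed and HP bar visibility.
; In range, it plays random attack montages, with OnAttack applying damage through a forward sphere trace.
; Damage updates the HP widget; death halts movement, notifies BP_BuildSysCharacter, then destroys the actor.
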(event `self.ReceiveBeginPlay`
  (`self.Init AI`)
  (`self.WaitAndMove`)
  (`self.Switch Mode` false))

(event `self.ReceiveTick`
  (params (DeltaSeconds :type "Float (single-precision)")))

(event `WaitAndMove`
  (bind _output_get (set `self.Waiting Period` (`KismetMathLibrary.RandomFloatInRange` 1.0 3.0)))
  (`KismetSystemLibrary.K2_SetTimerDelegate` (delegate `MoveTo`) _output_get))

(event `MoveTo`
  (bind _meleerange (`self.MeleeRange`))
  (bind _returnvalue (`AIBlueprintHelperLibrary.GetAIController` self))
  (if (not (`self.Dead`))
    (if (`self.InCombat`)
      (`AITask_MoveTo.AIMoveTo` _returnvalue (0.0 0.0 0.0) (`GameplayStatics.GetPlayerPawn` 0) (* _meleerange 0.25)
        (:`OnRequestFailed`
          _)
        (:`OnMoveFinished`
          _))
      (else
        (`AITask_MoveTo.AIMoveTo` _returnvalue (`NavigationSystemV1.K2_GetRandomReachablePointInRadius` (`self.Origin`) (`self.Radius`) null null) null (* _meleerange 0.5)
          (:`OnRequestFailed`
            _)
          (:`OnMoveFinished`
            _))))
    (if (`self.InCombat`)
      (if (`self.isTargetInRange`)
        (`self.ExecuteAttack`)
        (else
          (`self.MoveTo`)))
      (else
        (`self.WaitAndMove`)))))

(event `ExecuteAttack`
  (bind (_returnvalue_roll _returnvalue_pitch _returnvalue_yaw) (`KismetMathLibrary.BreakRotator` (`KismetMathLibrary.FindLookAtRotation` (`self.K2_GetActorLocation`) (`self.K2_GetActorLocation` (`GameplayStatics.GetPlayerPawn` 0)))))
  (if (not (`self.Dead`))
    (if (not (`self.IsAttacking`))
      (`KismetSystemLibrary.PrintString` "Executing Attack")
      (`self.K2_SetActorRotation` (`KismetMathLibrary.MakeRotator` 0.0 0.0 _returnvalue_yaw))
      (set `self.IsAttacking` true)
      (`|PlayMontage` (`self.Mesh`) (`KismetArrayLibrary.Array_Random` (`self.Attack Mons`))
        (:`OnCompleted`
          _)
        (:`OnBlendOut`
          _))
      (set `self.IsAttacking` false)
      (if (`self.isTargetInRange`)
        (`self.ExecuteAttack`)
        (else
          (`self.MoveTo`)))
      (else
        (`KismetSystemLibrary.PrintString` "Already Attacking")))))

(event `/Game/System/BP/BPI_Enemy.OnAttack`
  (bind _returnvalue (`self.K2_GetActorLocation`))
  (if (not (`self.Dead`))
    (bind (_outhit _returnvalue_2) (`KismetSystemLibrary.SphereTraceSingleForObjects` _returnvalue (+ _returnvalue (* (`self.GetActorForwardVector`) (`self.MeleeRange`))) 30.0 (`|MakeArray` "ObjectTypeQuery3" :!type "EObjectTypeQuery Enum")))
    (if _returnvalue_2
      (if (== (`.HitActor` (`GameplayStatics.BreakHitResult` _outhit)) (`GameplayStatics.GetPlayerPawn` 0))
        (`GameplayStatics.ApplyDamage` (`GameplayStatics.GetPlayerPawn` 0) (`self.Base Damage`) null self)))))

(event `/Game/System/BP/BPI_Enemy.Toggle Mark As Target`
  (params (Mark :type Boolean))
  (`SceneComponent.SetVisibility` (`self.Mark_Widget`) Mark false))

(event `OnDeath`
  (bind _charactermovement (`self.CharacterMovement`))
  (set `self.Dead` true)
  (`self.StopAnimMontage` null)
  (`MovementComponent.StopMovementImmediately` _charactermovement)
  (`Controller.StopMovement` (`AIBlueprintHelperLibrary.GetAIController` self))
  (`CharacterMovementComponent.DisableMovement` _charactermovement)
  (`SceneComponent.SetVisibility` (`self.HP_Widget`) false false)
  (`KismetSystemLibrary.Delay` 1.0)
  (bind _asbp_build_sys_charc (cast `/Game/System/BP/BP_BuildSysCharacter` (`GameplayStatics.GetPlayerPawn` 0)))
  (`/Game/System/BP/BP_BuildSysCharacter.On Enemy Die` _asbp_build_sys_charc)
  (`KismetSystemLibrary.Delay` 2.0)
  (`self.K2_DestroyActor`))

(event `self.ReceiveAnyDamage`
  (params (Damage :type "Float (single-precision)") (DamageType :type "DamageType Object Reference") (InstigatedBy :type "Controller Object Reference") (DamageCauser :type "Actor Object Reference"))
  (bind _maxhp (`self.MaxHP`))
  (bind _output_get (set `self.CurrentHP` (- (`self.CurrentHP`) Damage)))
  (`/Game/System/UMG/UI_HPBar.Set Percent` (`self.As UI HPBar`) (`KismetMathLibrary.FClamp` (/ _output_get _maxhp) 0.0 _maxhp))
  (if (<= (`self.CurrentHP`) 0.0)
    (`self.OnDeath`)))

(fn `Get Target Comp`
  (returns (TargetComp :type "SceneComponent Object Reference"))
  (return (`self.Mesh`)))

(fn `Init AI`
  (set `self.CurrentHP` (`self.MaxHP`))
  (bind _asui_hpbar (cast `/Game/System/UMG/UI_HPBar` (`WidgetComponent.GetUserWidgetObject` (`self.HP_Widget`))))
  (bind _output_get (set `self.As UI HPBar` _asui_hpbar))
  (`/Game/System/UMG/UI_HPBar.Set Percent` _output_get 1.0))

(fn `isDead`
  (returns (Dead :type Boolean))
  (return (`self.Dead`)))

(fn `isTargetInRange`
  (returns (ReturnValue :type Boolean))
  (return (<= (`self.GetDistanceTo` (`GameplayStatics.GetPlayerPawn` 0)) (`self.MeleeRange`))))

(fn `Switch Mode`
  (params (InCombat :type Boolean))
  (bind _output_get (set `self.InCombat` InCombat))
  (set `CharacterMovementComponent.MaxWalkSpeed` (`KismetMathLibrary.SelectFloat` (`self.Sprint Speed`) (`self.Walk Speed`) _output_get) (`self.CharacterMovement`))
  (`SceneComponent.SetVisibility` (`self.HP_Widget`) (`self.InCombat`) false))

(fn `UserConstructionScript`)