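; BP_PoisonBall is a poison projectile, attributed to the player, that damages what it hits.
; The construction script hands HomingTargetComponent to ProjectileMovement, or disables homing when that target is invalid.
; When Sphere1 overlaps any actor except player pawn 0, it applies BaseDamage with that pawn as causer, spawns a purple hit effect and destroys itself.
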(event `self.Sphere1.OnComponentBeginOverlap`
  (params (OverlappedComponent :type "PrimitiveComponent Object Reference") (OtherActor :type "Actor Object Reference") (OtherComp :type "PrimitiveComponent Object Reference") (OtherBodyIndex :type Integer) (bFromSweep :type Boolean) (SweepResult :type "HitResult Structure (by ref)"))
  (if (!= OtherActor (`GameplayStatics.GetPlayerPawn` 0))
    (`GameplayStatics.ApplyDamage` OtherActor (`self.Base Damage`) null (`GameplayStatics.GetPlayerPawn` 0))
    (`GameplayStatics.SpawnEmitterAtLocation` "/Game/MarketplaceAsset/MagicProjectilesVol2/Particles/Hits/P_Hit_Trail01_Purple.P_Hit_Trail01_Purple" (`self.K2_GetActorLocation`))
    (`self.K2_DestroyActor`)))

(fn `UserConstructionScript`
  (bind _projectilemovement (`self.ProjectileMovement`))
  (bind _homing_target_component (`self.Homing Target Component`))
  (`/Engine/EditorBlueprintResources/StandardMacros.IsValid` _homing_target_component
    (:`Is Valid`
      (set `ProjectileMovementComponent.HomingTargetComponent` _homing_target_component _projectilemovement))
    (:`Is Not Valid`
      (set `ProjectileMovementComponent.bIsHomingProjectile` false _projectilemovement))))