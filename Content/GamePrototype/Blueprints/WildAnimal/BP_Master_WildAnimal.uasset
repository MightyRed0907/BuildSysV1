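; BP_Master_WildAnimal is the wild animal master Blueprint, handling health, damage and death in multiplayer.
; The server sets health to maximum on BeginPlay and subtracts clamped damage, multicasting a hit animation that returns to looping idle afterwards.
; At zero health it multicasts the death animation, waits out its length, spawns the DeadBodyResource actor in place and destroys itself.
; Animations play directly on the skeletal mesh as sequence assets.
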(event `self.ReceiveBeginPlay`
  (`self.Initialize`))

(event `Initialize`
  ;[1 1 1] Initialize
  (if (`KismetSystemLibrary.IsServer`)
    (set `self.CurHealth` (`self.MaxHealth`))))

(event `Server_ReceiveDamage`
  (params (Damage :type "Float (double-precision)"))
  (bind _curhealth (`self.CurHealth`))
  (if (> _curhealth 0.0)
    (set `self.CurHealth` (`KismetMathLibrary.FClamp` (- _curhealth Damage) 0.0 (`self.MaxHealth`)))
    (if (<= (`self.CurHealth`) 0.0)
      (`self.Server_Death`)
      (else
        (`self.Multicast_PlayHitAnimation`)))))

(event `Server_Death`
  (`self.Multicast_PlayDeathAnimation`)
  (`KismetSystemLibrary.Delay` (`AnimSequenceBase.SequenceLength` (`self.DeathAnimSequence`)))
  (`|SpawnActorFromClass` (`self.DeadBodyResource`) (`self.GetTransform`) "Undefined" "OverrideRootScale" null null)
  (`self.K2_DestroyActor`))

(event `Multicast_PlayHitAnimation`
  (bind _hitanimsequence (`self.HitAnimSequence`))
  (`SkeletalMeshComponent.PlayAnimation` (`self.SkeletalMesh`) _hitanimsequence false)
  (`KismetSystemLibrary.Delay` (`AnimSequenceBase.SequenceLength` _hitanimsequence))
  (`SkeletalMeshComponent.PlayAnimation` (`self.SkeletalMesh`) (`self.IdleAnimSequence`) true))

(event `Multicast_PlayDeathAnimation`
  (`SkeletalMeshComponent.PlayAnimation` (`self.SkeletalMesh`) (`self.DeathAnimSequence`) false))

(fn `UserConstructionScript`)