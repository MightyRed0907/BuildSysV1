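; BP_DeadPlayerBag is a useable loot bag for a dead player's items, backed by a storage inventory component.
; Target events toggle custom depth on the bag mesh to highlight it while a player targets it.
; On spawn, the server runs an optional destroy timer that toggles the inventory of every player in the storage's player array, then destroys the bag.
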(event `/Game/GamePrototype/Blueprints/Other/Interfaces/BP_SurvivalInventoryInterface.Target`
  ;[0 0.5089 1] Client events
  ;;[1 1 1] Player target
  (`PrimitiveComponent.SetRenderCustomDepth` (`self.Loot Bag`) true))

(event `/Game/GamePrototype/Blueprints/Other/Interfaces/BP_SurvivalInventoryInterface.Not Target`
  ;[0 0.5089 1] Client events
  ;;[1 1 1] Not a player target
  (`PrimitiveComponent.SetRenderCustomDepth` (`self.Loot Bag`) false))

(event `On Spawned`
  (bind _player_array (`/Game/GamePrototype/Blueprints/Components/BP_StorageInventoryComponent.Player Array` (`self.StorageInventoryComponent`)))
  ;[0 1 0.09084] Server events
  ;;[1 1 1] On spawned
  (if (`self.Use Destroy Timer`)
    (`KismetSystemLibrary.Delay` (`self.Destroy Timer`))
    (if (> (`KismetArrayLibrary.Array_Length` _player_array) 0)
      (for _array_element _player_array
        (`/Engine/EditorBlueprintResources/StandardMacros.IsValid` _array_element
          (:`Is Valid`
            (`/Game/GamePrototype/Blueprints/Components/BP_PlayerInventoryComponent.Client Toggled Inventory` _array_element)))))
    (`self.K2_DestroyActor`)))

(fn `UserConstructionScript`)