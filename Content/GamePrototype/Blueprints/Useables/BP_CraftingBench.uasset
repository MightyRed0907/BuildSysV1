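; BP_CraftingBench is a usable crafting bench that players can target and interact with.
; Targeting toggles custom depth rendering on the bench mesh.
; Interacting toggles the player's inventory and registers the bench as that player component's interacted actor, also notifying the client.
; Query functions supply the prompt name, action text and E key icon, and report it as always interactable without a timed hold.
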(event `/Game/GamePrototype/Blueprints/Other/Interfaces/BP_SurvivalInventoryInterface.Target`
  ;[0 0.5089 1] Client events
  ;;[1 1 1] Player target
  (`PrimitiveComponent.SetRenderCustomDepth` (`self.Crafting Bench`) true))

(event `/Game/GamePrototype/Blueprints/Other/Interfaces/BP_SurvivalInventoryInterface.Not Target`
  ;[0 0.5089 1] Client events
  ;;[1 1 1] Not a player target
  (`PrimitiveComponent.SetRenderCustomDepth` (`self.Crafting Bench`) false))

(event `/Game/GamePrototype/Blueprints/Other/Interfaces/BP_SurvivalInventoryInterface.Interact`
  (params (`Player Component` :type "/Game/GamePrototype/Blueprints/Components/BP_PlayerInventoryComponent Object Reference"))
  (`/Game/GamePrototype/Blueprints/Components/BP_PlayerInventoryComponent.Client Toggled Inventory` `Player Component`)
  (set `/Game/GamePrototype/Blueprints/Components/BP_PlayerInventoryComponent.Interacted Actor` self `Player Component`)
  (`/Game/GamePrototype/Blueprints/Components/BP_PlayerInventoryComponent.Client Set Interacted Actor` `Player Component` self))

(fn `Interact Action`
  (returns (`Interact Action Text` :type Text))
  (return "INTERACT"))

(fn `Interact Input Brush`
  (returns (Brush :type "SlateBrush Structure"))
  (return (make `SlateBrush` (48.0 48.0) (struct) (struct :`SpecifiedColor` (struct :`R` 1.0 :`G` 1.0 :`B` 1.0 :`A` 1.0) :`ColorUseRule` "UseColor_Specified") (struct :`CornerRadii` (struct :`W` 1.0) :`Color` (struct :`SpecifiedColor` (struct) :`ColorUseRule` "UseColor_Specified") :`RoundingType` "HalfHeightRadius") "/Game/GamePrototype/Textures/Icons/Key_E_Icon.Key_E_Icon")))

(fn `Interact Name`
  (returns (`Instace Text` :type Text))
  (return "CRAFTING BENCH"))

(fn `Interact Time`
  (returns (`Interact Time` :type Boolean) (Time :type "Float (double-precision)"))
  (return false 0.0))

(fn `Interacting Action Text`
  (returns (Text :type Text))
  (return "INTERACTING..."))

(fn `Is Interactable`
  (returns (Interactable :type Boolean))
  (return true))

(fn `UserConstructionScript`)