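; BP_MasterConverter is a base interactable world object that hands player interaction to a ConvertInventoryComponent for item conversion.
; It answers interaction queries with prompt text, input brush, the component's storage name and an optional timed hold.
; A timed interaction spawns a sound at the actor, destroyed when the timer completes or cancels.
; On interact, it records itself as the player component's InteractedActor, then forwards the call to the inventory component.
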(event `/Game/GamePrototype/Blueprints/Other/Interfaces/BP_SurvivalInventoryInterface.Interact Done`
  (bind _interact_sound (`self.Interact Sound`))
  ;[0 0.5089 1] Client events
  ;;[1 1 1] Interaction timer done
  (`/Engine/EditorBlueprintResources/StandardMacros.IsValid` _interact_sound
    (:`Is Valid`
      (`ActorComponent.K2_DestroyComponent` _interact_sound))))

(event `/Game/GamePrototype/Blueprints/Other/Interfaces/BP_SurvivalInventoryInterface.Interact Cancelled`
  (bind _interact_sound (`self.Interact Sound`))
  ;[0 0.5089 1] Client events
  ;;[1 1 1] Interact timer cancelled
  (`/Engine/EditorBlueprintResources/StandardMacros.IsValid` _interact_sound
    (:`Is Valid`
      (`ActorComponent.K2_DestroyComponent` _interact_sound))))

(event `/Game/GamePrototype/Blueprints/Other/Interfaces/BP_SurvivalInventoryInterface.Interact`
  (params (`Player Component` :type "/Game/GamePrototype/Blueprints/Components/BP_PlayerInventoryComponent Object Reference"))
  ;[0 1 0.09084] Server events
  ;;[1 1 1] Interact event passed to component
  (set `/Game/GamePrototype/Blueprints/Components/BP_PlayerInventoryComponent.Interacted Actor` self `Player Component`)
  (`/Game/GamePrototype/Blueprints/Other/Interfaces/BP_SurvivalInventoryInterface.Interact` (`self.ConvertInventoryComponent`) `Player Component`))

(fn `Interact Action`
  (returns (`Interact Action Text` :type Text))
  (return (`self.Interact Action Text`)))

(fn `Interact Input Brush`
  (returns (Brush :type "SlateBrush Structure"))
  (return (`self.Interact Brush`)))

(fn `Interact Name`
  (returns (`Instace Text` :type Text))
  (return (`KismetTextLibrary.Conv_StringToText` (`/Game/GamePrototype/Blueprints/Components/BP_StorageInventoryComponent.Storage Name` (`self.ConvertInventoryComponent`)))))

(fn `Interact Time`
  (returns (`Interact Time` :type Boolean) (Time :type "Float (double-precision)"))
  ;[1 1 1] Interact time
  (if (`self.Use Interact Time`)
    (`/Engine/EditorBlueprintResources/StandardMacros.IsValid` (`self.Interact Timer Sound`)
      (:`Is Valid`
        ;;[1 1 1] Play the sound at location
        (bind _returnvalue (`GameplayStatics.SpawnSoundAtLocation` (`self.Interact Timer Sound`) (`self.K2_GetActorLocation`) (struct) 1.0 1.0 0.0 null null))
        (set `self.Interact Sound` _returnvalue)
        (return (`self.Use Interact Time`) (`self.Time To Interact`)))
      (:`Is Not Valid`
        (return (`self.Use Interact Time`) (`self.Time To Interact`))))
    (else
      (return false 0.0))))

(fn `Interacting Action Text`
  (returns (Text :type Text))
  (return (`self.Interact Timer Text`)))

(fn `Is Interactable`
  (returns (Interactable :type Boolean))
  (return true))

(fn `UserConstructionScript`)