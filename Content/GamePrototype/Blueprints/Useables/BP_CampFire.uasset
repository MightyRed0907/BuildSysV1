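; BP_CampFire is a useable campfire that can be lit and extinguished through interact animation events.
; Switching on shows the Fire component and plays FireSound, while switching off hides the fire and stops the sound, which is also stopped at BeginPlay.
; Target and NotTarget events toggle custom depth rendering on the CampFire component to mark it as the player's current target.
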(event `self.ReceiveBeginPlay`
  ;[0 1 0.09084] Server events
  ;;[1 1 1] Begin play
  (`AudioComponent.Stop` (`self.Fire Sound`)))

(event `/Game/GamePrototype/Blueprints/Other/Interfaces/BP_SurvivalInventoryInterface.Target`
  ;[0 0.5089 1] Client events
  ;;[1 1 1] Player target
  (`PrimitiveComponent.SetRenderCustomDepth` (`self.Camp Fire`) true))

(event `/Game/GamePrototype/Blueprints/Other/Interfaces/BP_SurvivalInventoryInterface.Switch Off Interact Animation`
  ;[0 1 0.09084] Server events
  ;;[1 1 1] Swtich off interact animation
  (`SceneComponent.SetVisibility` (`self.Fire`) false false)
  (`AudioComponent.Stop` (`self.Fire Sound`)))

(event `/Game/GamePrototype/Blueprints/Other/Interfaces/BP_SurvivalInventoryInterface.Not Target`
  ;[0 0.5089 1] Client events
  ;;[1 1 1] Not a player target
  (`PrimitiveComponent.SetRenderCustomDepth` (`self.Camp Fire`) false))

(event `/Game/GamePrototype/Blueprints/Other/Interfaces/BP_SurvivalInventoryInterface.Switch On Interact Animation`
  ;[0 1 0.09084] Server events
  ;;[1 1 1] Swtich on interact animation
  (`SceneComponent.SetVisibility` (`self.Fire`) true false)
  (`AudioComponent.Play` (`self.Fire Sound`) 0.0))

(fn `UserConstructionScript`
  (`parent.UserConstructionScript`))