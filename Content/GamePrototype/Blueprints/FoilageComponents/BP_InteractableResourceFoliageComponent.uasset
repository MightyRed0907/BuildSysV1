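; BP_InteractableResourceFoliageComponent is a foliage component that presents a resource to the interaction system.
; It overrides interaction query functions to return its own variables for interactable state, resource name, action text, input brush, and timed-interaction flag with duration.
; Each override calls its parent and discards the result.
; The file holds no gathering logic, and its BeginPlay and Tick events are disabled stubs.
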(fn `Interact Action`
  (returns (`Interact Action Text` :type Text))
  (`parent.Interact Action`)
  (return (`self.Interact Text`)))

(fn `Interact Input Brush`
  (returns (Brush :type "SlateBrush Structure"))
  (`parent.Interact Input Brush`)
  (return (`self.Interact Brush`)))

(fn `Interact Name`
  (returns (`Instace Text` :type Text))
  (`parent.Interact Name`)
  (return (`self.Resource Name`)))

(fn `Interact Time`
  (returns (`Interact Time` :type Boolean) (Time :type "Float (double-precision)"))
  (`parent.Interact Time`)
  (return (`self.Use Interact Time`) (`self.Timing Time`)))

(fn `Is Interactable`
  (returns (Interactable :type Boolean))
  (`parent.Is Interactable`)
  (return (`self.Interactable`)))