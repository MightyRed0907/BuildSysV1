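; BP_MasterHoldable is a networked base actor for held items, attached to a socket on the owning character's mesh.
; The server binds to the survival game mode's UpdateResources event to multicast re-attachment when new clients connect.
; A looping authority timer removes attachments and destroys the item when its inventory component or character becomes invalid.
; Interaction functions return empty defaults, so the base is not interactable.
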(event `self.ReceiveBeginPlay`
  (`/Engine/EditorBlueprintResources/ActorMacros.Switch Has Authority`
    (:`Authority`
      (bind _asbp_survival_game_mode (cast `/Game/GamePrototype/Blueprints/Characters/BP_SurvivalGameMode` (`GameplayStatics.GetGameMode`)))
      (add `/Game/GamePrototype/Blueprints/Characters/BP_SurvivalGameMode.Update Resources` _asbp_survival_game_mode (delegate `New Client Connected Bind`))
      (`KismetSystemLibrary.K2_SetTimer` null "Disconnect Check" 2.5 true))))

(event `Server New Client Connected`
  (`self.Multicast New Client` :!label _label))

(event `New Client Connected Bind`
  (goto _label))

(event `Multicast New Client`
  (bind _player_inventory_component (`self.Player Inventory Component`))
  (`/Engine/EditorBlueprintResources/StandardMacros.IsValid` _player_inventory_component
    (:`Is Valid`
      (`SceneComponent.K2_AttachToComponent` (`self.Attach Component`) (`Character.Mesh` (`/Game/GamePrototype/Blueprints/Components/BP_PlayerInventoryComponent.Master Character` _player_inventory_component)) (`self.Socket Name`) "SnapToTarget" "SnapToTarget" "SnapToTarget" true))))

(event `Destroy`
  ;[0 1 0.09084] Server events
  ;;[1 1 1] Destroy this actor
  (message `/Game/GamePrototype/Blueprints/Other/Interfaces/BP_SurvivalInventoryInterface.Remove All Attachments` self)
  (`self.K2_DestroyActor`))

(fn `Disconnect Check`
  (bind _player_inventory_component (`self.Player Inventory Component`))
  (`/Engine/EditorBlueprintResources/StandardMacros.IsValid` _player_inventory_component
    (:`Is Valid`
      (`/Engine/EditorBlueprintResources/StandardMacros.IsValid` (`/Game/GamePrototype/Blueprints/Components/BP_PlayerInventoryComponent.Master Character` _player_inventory_component)
        (:`Is Not Valid`
          _)))
    (:`Is Not Valid`
      _))
  (message `/Game/GamePrototype/Blueprints/Other/Interfaces/BP_SurvivalInventoryInterface.Remove All Attachments` self)
  (`self.K2_DestroyActor`))

(fn `Interact Action`
  (returns (`Interact Action Text` :type Text))
  (return ""))

(fn `Interact Input Brush`
  (returns (Brush :type "SlateBrush Structure"))
  (return))

(fn `Interact Name`
  (returns (`Instace Text` :type Text))
  (return ""))

(fn `Interact Time`
  (returns (`Interact Time` :type Boolean) (Time :type "Float (double-precision)"))
  (return false 0.0))

(fn `Interacting Action Text`
  (returns (Text :type Text))
  (return ""))

(fn `Is Interactable`
  (returns (Interactable :type Boolean))
  (return false))

(fn `UserConstructionScript`)