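; BP_Hammer is a holdable hammer that gives the player access to the building options menu.
; Its Q input handler shows the menu on key down and hides it on key up, via client toggle calls on the PlayerBuildingComponent reached through the PlayerInventoryComponent.
; Both actions are ignored while the inventory is open, and the construction script only calls its parent.
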(event `/Game/GamePrototype/Blueprints/Other/Interfaces/BP_SurvivalInventoryInterface.Q Input Action`
  (params (`Key Down` :type Boolean))
  ;[1 1 1] Open building menu
  (if (`/Game/GamePrototype/Blueprints/Components/BP_PlayerInventoryComponent.Inventory Open` (`self.Player Inventory Component`))
    _
    (elif `Key Down`
      (`/Game/GamePrototype/Blueprints/Components/BP_PlayerBuildingComponent.Client Toggle Building Options Menu` (`/Game/GamePrototype/Blueprints/Components/BP_PlayerInventoryComponent.Player Building Component` (`self.Player Inventory Component`)) true)
      (else
        (`/Game/GamePrototype/Blueprints/Components/BP_PlayerBuildingComponent.Client Toggle Building Options Menu` (`/Game/GamePrototype/Blueprints/Components/BP_PlayerInventoryComponent.Player Building Component` (`self.Player Inventory Component`)) false)))))

(fn `UserConstructionScript`
  (`parent.UserConstructionScript`))