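; Base-style interactable resource that the player harvests by hand through an interaction interface.
; On Interact it stores the passed player inventory component and, if interactable, calls ResourceCollected with that inventory's hands harvest amount.
; Interface overrides call their parent versions, then return the resource's own name, action text, input brush, interactable state and hold-time settings.
; Only the in-progress action text passes through the parent's value.
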(event `/Game/GamePrototype/Blueprints/Other/Interfaces/BP_SurvivalInventoryInterface.Interact`
  (params (`Player Component` :type "/Game/GamePrototype/Blueprints/Components/BP_PlayerInventoryComponent Object Reference"))
  (bind _player_inventory_component (`self.Player Inventory Component`))
  (set `self.Player Inventory Component` `Player Component`)
  (if (`self.Interactable`)
    (`self.Resource Collected` (`/Game/GamePrototype/Blueprints/Components/BP_PlayerInventoryComponent.Hands Harvest Amount` _player_inventory_component) _player_inventory_component)))

(fn `Interact Action`
  (returns (`Interact Action Text` :type Text))
  (`parent.Interact Action`)
  (return (`self.Interaction Text`)))

(fn `Interact Input Brush`
  (returns (Brush :type "SlateBrush Structure"))
  (`parent.Interact Input Brush`)
  (return (`self.Interaction Brush`)))

(fn `Interact Name`
  (returns (`Instace Text` :type Text))
  (`parent.Interact Name`)
  (return (`self.Resource Name`)))

(fn `Interact Time`
  (returns (`Interact Time` :type Boolean) (Time :type "Float (double-precision)"))
  (`parent.Interact Time`)
  (return (`self.Use Interact Time`) (`self.Interacting Time`)))

(fn `Interacting Action Text`
  (returns (Text :type Text))
  (bind _text (`parent.Interacting Action Text`))
  (return _text))

(fn `Is Interactable`
  (returns (Interactable :type Boolean))
  (`parent.Is Interactable`)
  (return (`self.Interactable`)))

(fn `UserConstructionScript`
  (`parent.UserConstructionScript`))