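; Wooden window build part that players can open and close, optionally restricted to players on its owners list.
; Server interaction runs through a 0.2-second DoOnce debounce, then multicasts a FlipFlop timeline that swings both shutters and swaps the prompt text.
; Targeting highlights the shutters via custom depth.
; Multicast destruction clears the meshes and spawns a destruction part, leaving older destructible-mesh logic unconnected.
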(event `/Game/GamePrototype/Blueprints/Other/Interfaces/BP_SurvivalInventoryInterface.Target`
  ;[0 0.5089 1] Client events
  ;;[1 1 1] Player target
  (`PrimitiveComponent.SetRenderCustomDepth` (`self.SM_Window_Door_L_Wood_01`) true)
  (`PrimitiveComponent.SetRenderCustomDepth` (`self.SM_Window_Door_R_Wood_01`) true))

(event `Multicast Interact`
  ;[1 0 0] Multicast events
  ;;[1 1 1] Multicast interact
  (`/Engine/EditorBlueprintResources/StandardMacros.FlipFlop`
    (:`A`
      (set `self.Interaction Text` "CLOSE WINDOW")
      (bind (_direction _minus_rotation _plus_rotation) (`Timeline|Window Animation` :!label _label)
        (:`Update`
          (`SceneComponent.K2_SetRelativeRotation` (`self.SM_Window_Door_R_Wood_01`) (`KismetMathLibrary.MakeRotator` 0.0 0.0 _minus_rotation) false false)
          (`SceneComponent.K2_SetRelativeRotation` (`self.SM_Window_Door_L_Wood_01`) (`KismetMathLibrary.MakeRotator` 0.0 0.0 _plus_rotation) false false))))
    (:`B`
      (set `self.Interaction Text` "OPEN WINDOW")
      (goto _label :!via `Reverse`))))

(event `/Game/GamePrototype/Blueprints/Other/Interfaces/BP_SurvivalInventoryInterface.Not Target`
  ;[0 0.5089 1] Client events
  ;;[1 1 1] Not a player target
  (`PrimitiveComponent.SetRenderCustomDepth` (`self.SM_Window_Door_L_Wood_01`) false)
  (`PrimitiveComponent.SetRenderCustomDepth` (`self.SM_Window_Door_R_Wood_01`) false))

(event `/Game/GamePrototype/Blueprints/Other/Interfaces/BP_SurvivalInventoryInterface.Interact`
  (params (`Player Component` :type "/Game/GamePrototype/Blueprints/Components/BP_PlayerInventoryComponent Object Reference"))
  ;[0 1 0.09084] Server events
  ;;[1 1 1] Interact
  (bind _output_get (set `self.Interacted Player Inventory` `Player Component`))
  (set `/Game/GamePrototype/Blueprints/Components/BP_PlayerInventoryComponent.Interacted Actor` self _output_get)
  (if (`self.Owner Required Interact`)
    (bind _return_value (`self.Check Owners` (`/Game/GamePrototype/Blueprints/Components/BP_PlayerBuildingComponent.Player Name` (`/Game/GamePrototype/Blueprints/Components/BP_PlayerInventoryComponent.Player Building Component` (`self.Interacted Player Inventory`)))))
    (if _return_value
      (`/Engine/EditorBlueprintResources/StandardMacros.DoOnce` false :!label _label_2
        (:`Completed`
          (`self.Multicast Interact`)
          (`KismetSystemLibrary.Delay` 0.2)
          (goto _label_2 :!via `Reset`))))
    (else
      (goto _label_2))))

(event `self.Multicast Destroy`
  ;[1 0 0] Multicast events
  ;;[1 1 1] Multicast destroy
  (set `self.Pending Destroy` true)
  (`StaticMeshComponent.SetStaticMesh` (`self.SM_Window_Door_L_Wood_01`) null)
  (`StaticMeshComponent.SetStaticMesh` (`self.SM_Window_Door_R_Wood_01`) null)
  (`StaticMeshComponent.SetStaticMesh` (`self.SM_Window_Frame_Wood_01`) null)
  (`self.SpawnDestructionBuildPart`))

(fn `UserConstructionScript`)