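; Survival game mode that syncs existing world state to each newly connected player after a short delay on PostLogin.
; It has master grids load for the joiner, resets wood door starting rotations and tells holdables a new client connected.
; It also passes deleted foliage instances to the resource manager to load for the joiner, updates resource collision, and finally spawns a resource manager if none exists.
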(event `self.K2_PostLogin`
  (params (NewPlayer :type "PlayerController Object Reference"))
  ;[1 1 1] On login to the server, load past created grids
  (set `self.New Connected Player` NewPlayer)
  (`KismetSystemLibrary.Delay` 2.0)
  (`|ExecutionSequence`
    (:`then_0`
      (bind _outactors (`GameplayStatics.GetAllActorsOfClass` "/Game/GamePrototype/Blueprints/BuildGrids/BP_MasterGrid.BP_MasterGrid_C"))
      (if (> (`KismetArrayLibrary.Array_Length` _outactors) 0)
        (for _array_element _outactors
          (`/Game/GamePrototype/Blueprints/BuildGrids/BP_MasterGrid.Server Load Grid On Join` _array_element (`self.New Connected Player`)))))
    (:`then_1`
      ;[1 1 1] Set door starting rotations
      (bind _outactors_2 (`GameplayStatics.GetAllActorsOfClass` "/Game/GamePrototype/Blueprints/BuildParts/BP_WoodDoorBuildPart.BP_WoodDoorBuildPart_C"))
      (if (> (`KismetArrayLibrary.Array_Length` _outactors_2) 0)
        (for _array_element_2 _outactors_2
          (`/Game/GamePrototype/Blueprints/BuildParts/BP_WoodDoorBuildPart.Server Set Starting Rotation` _array_element_2))))
    (:`then_2`
      ;[1 1 1] Server remove new clients deleted instances
      (bind _outactors_3 (`GameplayStatics.GetAllActorsOfClass` "/Game/GamePrototype/Blueprints/Resources/BP_ResourceManager.BP_ResourceManager_C"))
      (if (> (`KismetArrayLibrary.Array_Length` _outactors_3) 0)
        (`/Game/GamePrototype/Blueprints/Resources/BP_ResourceManager.Server Load Resources On Join` (`|GetArrayItem` _outactors_3) (`self.New Connected Player`) (`self.Deleted Foliage Instances`))))
    (:`then_3`
      ;[1 1 1] Update resource collision
      (`self.Update Resources`))
    (:`then_4`
      ;[1 1 1] Attach holdable to new client characters
      (bind _outactors_4 (`GameplayStatics.GetAllActorsOfClass` "/Game/GamePrototype/Blueprints/Holdables/BP_MasterHoldable.BP_MasterHoldable_C"))
      (if (> (`KismetArrayLibrary.Array_Length` _outactors_4) 0)
        (for _array_element_3 _outactors_4
          (`/Game/GamePrototype/Blueprints/Holdables/BP_MasterHoldable.Server New Client Connected` _array_element_3))))
    (:`then_5`
      ;[1 1 1] If no resource manager spawn found spawn one
      (bind _outactors_5 (`GameplayStatics.GetAllActorsOfClass` "/Game/GamePrototype/Blueprints/Resources/BP_ResourceManager.BP_ResourceManager_C"))
      (if (not (> (`KismetArrayLibrary.Array_Length` _outactors_5) 0))
        (`|SpawnActorFromClass` "/Game/GamePrototype/Blueprints/Resources/BP_ResourceManager.BP_ResourceManager_C" (`KismetMathLibrary.MakeTransform` (0.0 0.0 0.0)) "AlwaysSpawn" "OverrideRootScale" null null)))))

(fn `UserConstructionScript`)