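; Base player character that handles first-person, third-person and aim-down-sights cameras, body rotation, recoil, fall damage and death.
; Damage routes to the inventory component, which initializes on possession alongside the building component.
; Camera switches toggle mesh visibility and reattach held items, while timelines blend ADS transform and FOV from first person.
; Looping timers, Tick and RPCs update aim rotation, threshold-based body turning, fall tracking and server screen centre.
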(event `self.ReceivePossessed`
  (params (NewController :type "Controller Object Reference"))
  ;[0 1 0.09084] Server events
  ;;[1 1 1] Begin play
  (`self.Client Possessed`)
  (`KismetSystemLibrary.K2_SetTimerDelegate` (`|CreateDelegate` :!event `Timer`) 0.06 true :!label _label)
  (`/Engine/EditorBlueprintResources/ActorMacros.Switch Has Authority`
    (:`Authority`
      (`KismetSystemLibrary.K2_SetTimerDelegate` (`|CreateDelegate` :!event `Server Look At Rotation`) 0.06 true))
    (:`Remote`
      _))
  (`/Game/GamePrototype/Blueprints/Components/BP_PlayerInventoryComponent.Initialize Component` (`self.PlayerInventoryComponent`))
  (`/Game/GamePrototype/Blueprints/Components/BP_PlayerBuildingComponent.Initialize Component` (`self.PlayerBuildingComponent`))
  (if (`|EnumEquality` (`self.Camera View`) "NewEnumerator0")
    (`self.First Person`)))

(event `Client Possessed`
  ;[0 1 0.09084] Server events
  ;;[1 1 1] Begin play
  (goto _label))

(event `self.ReceiveAnyDamage`
  (params (Damage :type "Float (single-precision)") (DamageType :type "DamageType Object Reference") (InstigatedBy :type "Controller Object Reference") (DamageCauser :type "Actor Object Reference"))
  ;[0 1 0.09084] Server events
  ;;[1 1 1] Any damage
  (`/Game/GamePrototype/Blueprints/Other/Interfaces/BP_SurvivalInventoryInterface.Damage` (`self.PlayerInventoryComponent`) "NewEnumerator0" (`KismetMathLibrary.FTrunc` Damage) InstigatedBy DamageCauser))

(event `self.ReceiveBeginPlay`
  (bind _death_animations (`/Game/GamePrototype/Blueprints/Components/BP_PlayerInventoryComponent.Death Animations` (`self.PlayerInventoryComponent`)))
  ;[0 1 0.09084] Server events
  ;;[1 1 1] On Spawned Events
  (if (`self.Character Dead`)
    (`SkeletalMeshComponent.PlayAnimation` (`self.Mesh`) (`|GetArrayItem` _death_animations (`KismetMathLibrary.RandomIntegerInRange` 0 (`KismetArrayLibrary.Array_Length` _death_animations))) false)
    (`PrimitiveComponent.SetCollisionProfileName` (`self.CapsuleComponent`) "DeadPlayer" true)))

(event `Destroy Character`
  (params (Timer :type "Float (double-precision)"))
  ;[0 1 0.09084] Server events
  ;;[1 1 1] Kill character
  (`KismetSystemLibrary.Delay` (+ Timer 0.5))
  (`self.K2_DestroyActor`))

(event `/Game/GamePrototype/Blueprints/Other/Interfaces/BP_SurvivalInventoryInterface.Bleed Damage`
  (params (`Bleed Repeat Time` :type "Float (double-precision)") (`Bleed Length` :type "Float (double-precision)") (`Bleed Damage` :type Integer))
  ;[0 1 0.09084] Server events
  ;;[1 1 1] Bleed damage
  (message `/Game/GamePrototype/Blueprints/Other/Interfaces/BP_SurvivalInventoryInterface.Bleed Damage` (`self.PlayerInventoryComponent`) `Bleed Repeat Time` `Bleed Length` `Bleed Damage`))

(event `Server Set Camera View`
  (params (`Camera view` :type "/Game/GamePrototype/Blueprints/Other/Enums/E_CameraView Enum" :default "NewEnumerator0"))
  ;[0 1 0.09084] Server events
  ;;[1 1 1] Server set camera view
  (set `self.Camera View` `Camera view`))

(event `/Game/GamePrototype/Blueprints/Other/Interfaces/BP_SurvivalInventoryInterface.Damage`
  (params (Hitbox :type "/Game/GamePrototype/Blueprints/Other/Enums/E_HitboxType Enum" :default "NewEnumerator0") (Damage :type Integer) (`Damage Owner` :type "Actor Object Reference") (`Damage Cause` :type "Actor Object Reference"))
  ;[0 1 0.09084] Server events
  ;;[1 1 1] Damage
  (`/Game/GamePrototype/Blueprints/Other/Interfaces/BP_SurvivalInventoryInterface.Damage` (`self.PlayerInventoryComponent`) Hitbox Damage `Damage Owner` `Damage Cause`))

(event `Multicast Stop Character Movement`
  ;[1 0 0] Multicast events
  ;;[1 1 1] Multicast stop character movement
  (`MovementComponent.StopMovementImmediately` (`self.CharacterMovement`)))

(event `Third Person`
  (bind _asbp_master_holdable (cast `/Game/GamePrototype/Blueprints/Holdables/BP_MasterHoldable` (`self.Held Actor`) :!pure true))
  ;[0 0.5089 1] Client events
  ;;[1 1 1] Client third person camera
  (`/Game/GamePrototype/Blueprints/Components/BP_PlayerInventoryComponent.Client Camera View` (`self.PlayerInventoryComponent`) "NewEnumerator1")
  (bind _output_get (set `self.Camera View` "NewEnumerator1"))
  (`self.Server Set Camera View` _output_get)
  (`ActorComponent.Deactivate` (`self.FP Camera`))
  (`ActorComponent.Activate` (`self.TP Camera`) true)
  (`PrimitiveComponent.SetOwnerNoSee` (`self.Head`) false)
  (`PrimitiveComponent.SetOwnerNoSee` (`self.Legs`) false)
  (`PrimitiveComponent.SetOwnerNoSee` (`self.Backpack`) false)
  (`PrimitiveComponent.SetOwnerNoSee` (`self.Feet`) false)
  (`PrimitiveComponent.SetOwnerNoSee` (`self.Chest`) false)
  (`PrimitiveComponent.SetOwnerNoSee` (`self.Mesh`) false)
  (`SceneComponent.SetVisibility` (`self.FP Viewport Mesh`) false false)
  (`/Engine/EditorBlueprintResources/StandardMacros.IsValid` (`self.Held Actor`)
    (:`Is Valid`
      (`SceneComponent.K2_AttachToComponent` (`/Game/GamePrototype/Blueprints/Holdables/BP_MasterHoldable.Attach Component` _asbp_master_holdable) (`self.Mesh`) (`/Game/GamePrototype/Blueprints/Holdables/BP_MasterHoldable.Socket Name` _asbp_master_holdable) "SnapToTarget" "SnapToTarget" "SnapToTarget" true))))

(event `First Person`
  (bind _asbp_master_holdable (cast `/Game/GamePrototype/Blueprints/Holdables/BP_MasterHoldable` (`self.Held Actor`) :!pure true))
  ;[0 0.5089 1] Client events
  ;;[1 1 1] Client first person camera
  (`/Game/GamePrototype/Blueprints/Components/BP_PlayerInventoryComponent.Client Camera View` (`self.PlayerInventoryComponent`) "NewEnumerator0")
  (bind _output_get (set `self.Camera View` "NewEnumerator0"))
  (`self.Server Set Camera View` _output_get)
  (`ActorComponent.Deactivate` (`self.TP Camera`))
  (`ActorComponent.Activate` (`self.FP Camera`) true)
  (`PrimitiveComponent.SetOwnerNoSee` (`self.Head`) true)
  (`PrimitiveComponent.SetOwnerNoSee` (`self.Legs`) true)
  (`PrimitiveComponent.SetOwnerNoSee` (`self.Backpack`) true)
  (`PrimitiveComponent.SetOwnerNoSee` (`self.Feet`) true)
  (`PrimitiveComponent.SetOwnerNoSee` (`self.Chest`) true)
  (`PrimitiveComponent.SetOwnerNoSee` (`self.Mesh`) true)
  (`SceneComponent.SetVisibility` (`self.FP Viewport Mesh`) true false)
  (`/Engine/EditorBlueprintResources/StandardMacros.IsValid` (`self.Held Actor`)
    (:`Is Valid`
      (`self.K2_DetachFromActor` (`self.Held Actor`) "KeepRelative" "KeepRelative" "KeepRelative")
      (`SceneComponent.K2_AttachToComponent` (`/Game/GamePrototype/Blueprints/Holdables/BP_MasterHoldable.Attach Component` _asbp_master_holdable) (`self.FP Viewport Mesh`) (`/Game/GamePrototype/Blueprints/Holdables/BP_MasterHoldable.Socket Name` _asbp_master_holdable) "SnapToTarget" "SnapToTarget" "SnapToTarget" true))))

(event `Timer`
  (bind (_returnvalue_roll _returnvalue_pitch _returnvalue_yaw) (`KismetMathLibrary.BreakRotator` (`self.K2_GetActorRotation`)))
  (bind (_returnvalue_roll_2 _returnvalue_pitch_2 _returnvalue_yaw_2) (`KismetMathLibrary.BreakRotator` (`self.GetControlRotation`)))
  (bind (_returnvalue_roll_3 _returnvalue_pitch_3 _returnvalue_yaw_3) (`KismetMathLibrary.BreakRotator` (`KismetMathLibrary.NormalizedDeltaRotator` (`KismetMathLibrary.MakeRotator` 0.0 0.0 _returnvalue_yaw_2) (`KismetMathLibrary.MakeRotator` 0.0 0.0 _returnvalue_yaw))))
  (bind (_velocity_x _velocity_y _velocity_z) (`KismetMathLibrary.BreakVector` (`MovementComponent.Velocity` (`self.CharacterMovement`))))
  ;[0 0.5089 1] Client events
  ;;[1 1 1] Set all character rotations
  (`|ExecutionSequence`
    (:`then_0`
      (`/Engine/EditorBlueprintResources/ActorMacros.Switch Has Authority`
        (:`Authority`
          (if (`self.IsLocallyControlled`)
            (set `self.Look At Rotation` (`self.GetControlRotation`))))
        (:`Remote`
          (`/Engine/EditorBlueprintResources/StandardMacros.IsValid` (`self.GetController`)
            (:`Is Valid`
              (set `self.Look At Rotation` (`self.GetControlRotation`)))))))
    (:`then_1`
      (if (or (`self.Rotate Character`) (>= (`KismetMathLibrary.Abs` _returnvalue_yaw_3) 80.0))
        (set `CharacterMovementComponent.bUseControllerDesiredRotation` true (`self.CharacterMovement`))
        (set `self.Rotate Character` (not (`KismetMathLibrary.NearlyEqual_FloatFloat` _returnvalue_yaw_3 0.0 2.0)))
        (else
          (set `CharacterMovementComponent.bUseControllerDesiredRotation` false (`self.CharacterMovement`)))))
    (:`then_2`
      (if (`self.Fall Damage `)
        (`/Engine/EditorBlueprintResources/ActorMacros.Switch Has Authority`
          (:`Authority`
            (if (`NavMovementComponent.IsFalling` (`self.CharacterMovement`))
              (if (<= _velocity_z (`self.Fall Damage Velocity`))
                (set `self.Damage Velocity Reached` true)
                (`/Engine/EditorBlueprintResources/StandardMacros.DoOnce` false :!label _label_2
                  (:`Completed`
                    (set `self.Start Fall Time` (`GameplayStatics.GetRealTimeSeconds`))))))))))
    (:`then_3`
      (`/Engine/EditorBlueprintResources/StandardMacros.IsValid` (`self.Held Actor`)
        (:`Is Valid`
          (if (`self.IsLocallyControlled`)
            (`self.Server Set Screen Centre` (`SceneComponent.K2_GetComponentLocation` (select `bool` (`/Game/GamePrototype/Blueprints/Components/BP_PlayerInventoryComponent.ADS` (`self.PlayerInventoryComponent`)) :`false` (select `/Game/GamePrototype/Blueprints/Other/Enums/E_CameraView` (`/Game/GamePrototype/Blueprints/Components/BP_PlayerInventoryComponent.Camera View` (`self.PlayerInventoryComponent`)) :`NewEnumerator0` (`self.FP Camera`) :`NewEnumerator1` (`self.TP Camera`)) :`true` (`self.ADS Camera`) :!type "SceneComponent Object Reference")))))))
    (:`then_4`
      (if (> (`KismetMathLibrary.VSize` (`self.GetVelocity`)) 0.0)
        (set `self.Rotate Character` true)
        (goto _label_3 :!via `Reset`)
        (else
          (`/Engine/EditorBlueprintResources/StandardMacros.DoOnce` false :!label _label_3
            (:`Completed`
              (set `self.Rotate Character` false))))))))

(event `Reset Fall Damage`
  ;[0 0.5089 1] Client events
  ;;[1 1 1] Set all character rotations
  (set `self.Start Fall Time` 0.0)
  (set `self.End Fall Time` 0.0)
  (set `self.Damage Velocity Reached` false)
  (goto _label_2 :!via `Reset`))

(event `self.ReceiveTick`
  (params (DeltaSeconds :type "Float (single-precision)"))
  ;[0 0.5089 1] Client events
  ;;[1 1 1] Local AO rotation
  (`/Engine/EditorBlueprintResources/ActorMacros.Switch Has Authority`
    (:`Authority`
      (if (`self.IsLocallyControlled`)
        (set `self.Look At Rotation` (`self.GetControlRotation`) :!label _label_4)))
    (:`Remote`
      (`/Engine/EditorBlueprintResources/StandardMacros.IsValid` (`self.GetController`)
        (:`Is Valid`
          (goto _label_4))))))

(event `self.OnLanded`
  (params (Hit :type "HitResult Structure (by ref)"))
  ;[0 1 0.09084] Server events
  ;;[1 1 1] On landed
  (if (`self.Fall Damage `)
    (if (`self.Damage Velocity Reached`)
      (set `self.End Fall Time` (`GameplayStatics.GetRealTimeSeconds`))
      (if (> (- (`self.End Fall Time`) (`self.Start Fall Time`)) (`self.Start Fall Damage Time`))
        (`/Game/GamePrototype/Blueprints/Components/BP_PlayerInventoryComponent.Deduct Health` (`self.PlayerInventoryComponent`) (`KismetMathLibrary.FTrunc` (* (`.ReturnValue` (`KismetMathLibrary.FMod` (- (`self.End Fall Time`) (`self.Start Fall Time`)) (`self.Fall Damage Increese Time`))) (`self.Fall Damage`))))
        (`self.Reset Fall Damage`)
        (else
          (`self.Reset Fall Damage`))))))

(event `Client Set Speed`
  (params (Speed :type "Float (double-precision)"))
  ;[0 0.5089 1] Client events
  ;;[1 1 1] Client set character speed
  (set `CharacterMovementComponent.MaxWalkSpeed` Speed (`self.CharacterMovement`)))

(event `Client Recoil`
  (params (`Weapon Recoil` :type "/Game/GamePrototype/Blueprints/Other/S_WeaponRecoil Structure"))
  (bind (_yawmin _yawmax _pitchmin _pitchmax) (break `/Game/GamePrototype/Blueprints/Other/S_WeaponRecoil` `Weapon Recoil`))
  ;[0 0.5089 1] Client events
  ;;[1 1 1] Client recoil
  (`self.AddControllerYawInput` (`KismetMathLibrary.RandomFloatInRange` _yawmin _yawmax))
  (`self.AddControllerPitchInput` (`KismetMathLibrary.RandomFloatInRange` _pitchmin _pitchmax)))

(event `Multicast Look At Rotation`
  (params (Rotation :type "Float (double-precision)"))
  (bind (_returnvalue_roll _returnvalue_pitch) (`KismetMathLibrary.BreakRotator` (`self.GetBaseAimRotation`)))
  ;[1 0 0] Multicast events
  ;;[1 1 1] Multicast look at rotation
  (if (not (`self.IsLocallyControlled`))
    (set `self.Look At Rotation` (`KismetMathLibrary.MakeRotator` _returnvalue_roll _returnvalue_pitch Rotation))))

(event `Server Look At Rotation`
  ;[0 1 0.09084] Server events
  ;;[1 1 1] Server look at rotation
  (`self.Multicast Look At Rotation` (.yaw (`self.GetBaseAimRotation`))))

(event `Client Zoom In ADS`
  ;[0 0.5089 1] Client events
  ;;[1 1 1] Client zoom In ADS
  (`SceneComponent.K2_SetRelativeTransform` (`self.ADS Socket`) (`/Game/GamePrototype/Blueprints/Holdables/BP_MasterWeapon.Return ADS Camera` (cast `/Game/GamePrototype/Blueprints/Holdables/BP_MasterWeapon` (`self.Held Actor`) :!pure true)) false false)
  (`ActorComponent.Deactivate` (`self.FP Camera`))
  (if (`/Game/GamePrototype/Blueprints/Components/BP_PlayerInventoryComponent.Was Third Person` (`self.PlayerInventoryComponent`))
    (`ActorComponent.Activate` (`self.ADS Camera`) true)
    (set `self.Camera Animation` false)
    (`SceneComponent.K2_SetWorldTransform` (`self.ADS Camera`) (`SceneComponent.K2_GetComponentToWorld` (`self.ADS Socket`)) false false)
    (`SceneComponent.K2_AttachToComponent` (`self.ADS Camera`) (`self.ADS Socket`) "None" "SnapToTarget" "SnapToTarget" "SnapToTarget" true)
    (`CameraComponent.SetFieldOfView` (`self.ADS Camera`) (`/Game/GamePrototype/Blueprints/Holdables/BP_MasterRangeWeapon.ADS FOV` (cast `/Game/GamePrototype/Blueprints/Holdables/BP_MasterRangeWeapon` (`self.Held Actor`) :!pure true)))
    (if (`/Game/GamePrototype/Blueprints/Components/BP_PlayerInventoryComponent.Equipping` (`self.PlayerInventoryComponent`))
      (`/Game/GamePrototype/Blueprints/Components/BP_PlayerInventoryComponent.Client Exit Aimed` (`self.PlayerInventoryComponent`) true))
    (else
      (`ActorComponent.Activate` (`self.ADS Camera`) true)
      (set `self.Camera Animation` true)
      (bind (_direction _zoom_in) (`Timeline|Zoom In` :!via `PlayFromStart` :!label _label_5)
        (:`Update`
          (if (`/Game/GamePrototype/Blueprints/Components/BP_PlayerInventoryComponent.Equipping` (`self.PlayerInventoryComponent`))
            (`|ExecutionSequence`
              (:`then_0`
                (`self.Stop FP Zoom In ADS`))
              (:`then_1`
                (`/Game/GamePrototype/Blueprints/Components/BP_PlayerInventoryComponent.Client Exit Aimed` (`self.PlayerInventoryComponent`) true)))
            (else
              (`SceneComponent.K2_SetWorldTransform` (`self.ADS Camera`) (`KismetMathLibrary.TLerp` (`SceneComponent.K2_GetComponentToWorld` (`self.ADS Camera`)) (`SceneComponent.K2_GetComponentToWorld` (`self.ADS Socket`)) _zoom_in) false false)
              (`CameraComponent.SetFieldOfView` (`self.ADS Camera`) (`KismetMathLibrary.Lerp` 90.0 (`/Game/GamePrototype/Blueprints/Holdables/BP_MasterRangeWeapon.ADS FOV` (cast `/Game/GamePrototype/Blueprints/Holdables/BP_MasterRangeWeapon` (`self.Held Actor`) :!pure true)) _zoom_in)))))
        (:`Finished`
          (set `self.Camera Animation` false)
          (`SceneComponent.K2_AttachToComponent` (`self.ADS Camera`) (`self.ADS Socket`) "None" "SnapToTarget" "SnapToTarget" "SnapToTarget" true))))))

(event `Stop FP Zoom In ADS`
  ;[0 0.5089 1] Client events
  ;;[1 1 1] Client zoom In ADS
  (goto _label_5 :!via `Stop`))

(event `Client Zoom Out ADS`
  ;[0 0.5089 1] Client events
  ;;[1 1 1] Client zoom out ADS
  (if (`/Game/GamePrototype/Blueprints/Components/BP_PlayerInventoryComponent.Was Third Person` (`self.PlayerInventoryComponent`))
    (`SceneComponent.K2_SetWorldTransform` (`self.ADS Camera`) (`SceneComponent.K2_GetComponentToWorld` (`self.FP Camera`)) false false)
    (set `self.Camera Animation` false)
    (`ActorComponent.Deactivate` (`self.ADS Camera`))
    (if (`/Game/GamePrototype/Blueprints/Components/BP_PlayerInventoryComponent.Was Third Person` (`self.PlayerInventoryComponent`))
      (`self.Third Person`)
      (else
        (`self.First Person`)))
    (else
      (set `self.Camera Animation` true)
      (bind (_direction _zoom_out) (`Timeline|Zoom Out` :!via `PlayFromStart`)
        (:`Update`
          (`CameraComponent.SetFieldOfView` (`self.ADS Camera`) (`KismetMathLibrary.Lerp` 75.0 90.0 _zoom_out))
          (`SceneComponent.K2_SetWorldTransform` (`self.ADS Camera`) (`KismetMathLibrary.TLerp` (`SceneComponent.K2_GetComponentToWorld` (`self.ADS Camera`)) (`SceneComponent.K2_GetComponentToWorld` (`self.FP Camera`)) _zoom_out) false false))
        (:`Finished`
          (set `self.Camera Animation` false)
          (`ActorComponent.Deactivate` (`self.ADS Camera`))
          (if (`/Game/GamePrototype/Blueprints/Components/BP_PlayerInventoryComponent.Was Third Person` (`self.PlayerInventoryComponent`))
            (`self.Third Person`)
            (else
              (`self.First Person`))))))))

(event `Server Set Screen Centre`
  (params (Center :type "Vector Structure"))
  ;[0 1 0.09084] Server events
  ;;[1 1 1] Server set screen centre
  (set `self.Screen Centre` Center))

(fn `Interact Action`
  (returns (`Interact Action Text` :type Text))
  (return ""))

(fn `Interact Input Brush`
  (returns (Brush :type "SlateBrush Structure"))
  (return))

(fn `Interact Name`
  (returns (`Instace Text` :type Text))
  (return ""))

(fn `Interact Time`
  (returns (`Interact Time` :type Boolean) (Time :type "Float (double-precision)"))
  (return false 0.0))

(fn `Interacting Action Text`
  (returns (Text :type Text))
  (return ""))

(fn `Is Interactable`
  (returns (Interactable :type Boolean))
  (return false))

(fn `UserConstructionScript`
  (`SkinnedMeshComponent.SetLeaderPoseComponent` (`self.Head`) (`self.Mesh`) false)
  (`SkinnedMeshComponent.SetLeaderPoseComponent` (`self.Backpack`) (`self.Mesh`) false)
  (`SkinnedMeshComponent.SetLeaderPoseComponent` (`self.Chest`) (`self.Mesh`) false)
  (`SkinnedMeshComponent.SetLeaderPoseComponent` (`self.Legs`) (`self.Mesh`) false)
  (`SkinnedMeshComponent.SetLeaderPoseComponent` (`self.Feet`) (`self.Mesh`) false))