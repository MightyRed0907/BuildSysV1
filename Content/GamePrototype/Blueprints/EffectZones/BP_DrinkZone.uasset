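; BP_DrinkZone is an interactable zone that changes the player's thirst when used.
; Interact adds a configurable drink amount to the inventory component's Thirst, clamped between 0 and 100, then sends a client notification.
; Multicast events play the drink sound and briefly ignore the Visibility channel on the zone, creating a reuse cooldown.
; Interface functions supply the prompt text, icon and timing, and construction sets in-game visibility.
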(event `Multicast Sound`
  ;[1 1 1] Multicast the drink sound
  (`GameplayStatics.PlaySoundAtLocation` (`self.Drink Sound`) (`self.K2_GetActorLocation`) (struct) 1.0 1.0 0.0 null null null null))

(event `Multicast Collision`
  ;[1 1 1] Block interaction
  (`PrimitiveComponent.SetCollisionResponseToChannel` (`self.Drink Zone`) "ECC_Visibility" "ECR_Ignore")
  ;[1 1 1] After delay allow interaction
  (`KismetSystemLibrary.Delay` (`self.Delay Time`))
  (`PrimitiveComponent.SetCollisionResponseToChannel` (`self.Drink Zone`) "ECC_Visibility" "ECR_Block"))

(event `/Game/GamePrototype/Blueprints/Other/Interfaces/BP_SurvivalInventoryInterface.Interact`
  (params (`Player Component` :type "/Game/GamePrototype/Blueprints/Components/BP_PlayerInventoryComponent Object Reference"))
  (bind _returnvalue (+ (`self.Drink Amount`) (`/Game/GamePrototype/Blueprints/Components/BP_PlayerInventoryComponent.Thirst` (`self.Player Inventory Component`))))
  (set `self.Player Inventory Component` `Player Component`)
  ;[1 1 1] Check if item effects thirst value
  (if (not (== (`self.Drink Amount`) 0.0))
    ;[1 1 1] If the item effects thirst, then apply effect and update clients thirst stat
    (if (>= _returnvalue 100.0)
      (set `/Game/GamePrototype/Blueprints/Components/BP_PlayerInventoryComponent.Thirst` 100.0 (`self.Player Inventory Component`))
      (elif (<= _returnvalue 0.0)
        (set `/Game/GamePrototype/Blueprints/Components/BP_PlayerInventoryComponent.Thirst` 0.0 (`self.Player Inventory Component`))
        (else
          (set `/Game/GamePrototype/Blueprints/Components/BP_PlayerInventoryComponent.Thirst` _returnvalue (`self.Player Inventory Component`))))))
  ;[1 1 1] Notification
  (`/Game/GamePrototype/Blueprints/Components/BP_PlayerInventoryComponent.Client Create Notification` :`self` (`self.Player Inventory Component`) :`Notification Type` "NewEnumerator4" :`Warning Text` (`self.Notification Text`) :`Notification Image` true)
  ;[1 1 1] Play sound
  (`self.Multicast Sound`)
  (`self.Multicast Collision`))

(fn `Interact Action`
  (returns (`Interact Action Text` :type Text))
  (return (`self.Interaction Action Text`)))

(fn `Interact Input Brush`
  (returns (Brush :type "SlateBrush Structure"))
  (return (`self.Interaction Icon`)))

(fn `Interact Name`
  (returns (`Instace Text` :type Text))
  (return (`self.Interaction Name`)))

(fn `Interact Time`
  (returns (`Interact Time` :type Boolean) (Time :type "Float (double-precision)"))
  (return (`self.Use Interact Time`) (`self.Interaction Time`)))

(fn `Interacting Action Text`
  (returns (Text :type Text))
  (return (`self.Interaction Time Text`)))

(fn `Is Interactable`
  (returns (Interactable :type Boolean))
  (return true))

(fn `UserConstructionScript`
  (`SceneComponent.SetHiddenInGame` (`self.Drink Zone`) (not (`self.Show Drink Zone In Game`)) false))